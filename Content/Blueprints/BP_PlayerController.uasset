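; Player controller that owns the local player's HUD and scoreboard widgets and pushes gameplay values into them.
; On BeginPlay it creates both widgets and starts a looping timer that formats the GameState time as minutes and seconds.
; Events update health, bullets and four directional damage reticles faded by timelines, while scoreboard input shows the board, rebuilding its list if player count differs.
; Possession resets displayed health after a tiny delay, working around a not-yet-valid HUD reference.
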(event `self.ReceiveBeginPlay`
  (if (`self.IsLocalPlayerController`)
    (bind _returnvalue (`|CreateWidget` "/Game/Blueprints/HUD/BP_HUD.BP_HUD_C" self))
    (bind _output_get (set `self.HUDRef` _returnvalue))
    (`UserWidget.AddToViewport` _output_get 0)
    (bind _returnvalue_2 (`|CreateWidget` "/Game/Blueprints/HUD/ScoreBoard/BP_Scoreboard.BP_Scoreboard_C" self))
    (bind _output_get_2 (set `self.ScoreboardRef` _returnvalue_2))
    (`UserWidget.AddToViewport` _output_get_2 0)
    (`Widget.SetVisibility` _output_get_2 "Hidden")
    (bind _asbp_game_state (cast `/Game/Blueprints/BP_GameState` (`GameplayStatics.GetGameState`))
      (:`then`
        (set `self.GameStateRef` _asbp_game_state)
        (`KismetSystemLibrary.K2_SetTimer` null "UpdateTimerText" 0.1 true))
      (:`CastFailed`
        (`KismetSystemLibrary.PrintString` "Cast to GameState failed in playercontroller")))))

(event `UpdateHealthText`
  (params (Health :type Integer))
  (bind _healthbar (`/Game/Blueprints/HUD/BP_HUD.HealthBar` (`self.HUDRef`)))
  (set `TextBlock.Text` (`KismetTextLibrary.Conv_IntToText` Health) (`/Game/Blueprints/HUD/BP_HUD.Health` (`self.HUDRef`)))
  (set `ProgressBar.Percent` (`KismetMathLibrary.SafeDivide` (`KismetMathLibrary.Conv_IntToDouble` Health) 100.0) _healthbar)
  (if (<= Health 20)
    (set `ProgressBar.FillColorAndOpacity` (`self.RedColor`) _healthbar)
    (else
      (set `ProgressBar.FillColorAndOpacity` (`self.WhiteColor`) _healthbar))))

(event `EnhancedInput|/Game/Blueprints/Inputs/IA_Scoreboard`
  (params (ActionValue :type Boolean) (ElapsedSeconds :type "Float (double-precision)") (TriggeredSeconds :type "Float (double-precision)") (InputAction :type "InputAction Object Reference" :default "/Game/Blueprints/Inputs/IA_Scoreboard.IA_Scoreboard"))
  (bind _scoreboardref (`self.ScoreboardRef`))
  (:`Triggered`
    (if ActionValue
      (`Widget.SetVisibility` _scoreboardref "Visible")
      (if (!= (`KismetArrayLibrary.Array_Length` (`GameStateBase.PlayerArray` (cast `/Game/Blueprints/BP_GameState` (`GameplayStatics.GetGameState`) :!pure true))) (`PanelWidget.GetChildrenCount` (`/Game/Blueprints/HUD/ScoreBoard/BP_Scoreboard.PlayerListInScoreboard` (`self.ScoreboardRef`))))
        (`/Game/Blueprints/HUD/ScoreBoard/BP_Scoreboard.UpdatePlayerListInScoreboard` _scoreboardref)
        (else
          (`/Game/Blueprints/HUD/ScoreBoard/BP_Scoreboard.UpdateScoreboard` _scoreboardref)))
      (else
        (`Widget.SetVisibility` _scoreboardref "Hidden")))))

(event `UpdateTimerText`
  (bind _time (`/Game/Blueprints/BP_GameState.GetTime` (`self.GameStateRef`)))
  (bind _returnvalue (mod _time 60))
  (if (< _returnvalue 10)
    (bind _returnvalue_2 (/ _time 60))
    (set `TextBlock.Text` (`|FormatText` "{Mins} : 0{Sec}" _returnvalue_2 _returnvalue) (`/Game/Blueprints/HUD/BP_HUD.Timer` (`self.HUDRef`)))
    (else
      (set `TextBlock.Text` (`|FormatText` "{Mins} : {Sec}" _returnvalue_2 _returnvalue) (`/Game/Blueprints/HUD/BP_HUD.Timer` (`self.HUDRef`))))))

(event `self.ReceivePossess`
  (params (PossessedPawn :type "Pawn Object Reference"))
  (`KismetSystemLibrary.K2_SetTimerDelegate` (delegate `UpdateHealthAfterRespawn`) 1e-05) ; Need a small delay because the HUDRef isn't valid instantly for some reason
)

(event `UpdateHealthAfterRespawn`
  (`/Engine/EditorBlueprintResources/StandardMacros.IsValid` (`self.HUDRef`)
    (:`Is Valid`
      (`self.UpdateHealthText` 100))))

(event `UpdateBullets`
  (params (Bullets :type Integer))
  (set `TextBlock.Text` (`KismetTextLibrary.Conv_IntToText` Bullets) (`/Game/Blueprints/HUD/BP_HUD.Bullets` (`self.HUDRef`))))

(event `RightDamageReticle`
  (params (`In Color and Opacity A` :type "Float (single-precision)"))
  (bind (_direction _multiplier) (`Timeline|DamageReticleDisappeardRight` :!via `PlayFromStart`)
    (:`Update`
      (`Image.SetColorAndOpacity` (`/Game/Blueprints/HUD/BP_HUD.Right_Reticle` (`self.HUDRef`)) (make `LinearColor` 1.0 1.0 1.0 (* _multiplier `In Color and Opacity A`))))))

(event `TopDamageReticle`
  (params (`In Color and Opacity A` :type "Float (single-precision)"))
  (bind (_direction _multiplier) (`Timeline|DamageReticleDisappeardTop` :!via `PlayFromStart`)
    (:`Update`
      (`Image.SetColorAndOpacity` (`/Game/Blueprints/HUD/BP_HUD.Top_Reticle` (`self.HUDRef`)) (make `LinearColor` 1.0 1.0 1.0 (* _multiplier `In Color and Opacity A`))))))

(event `LeftDamageReticle`
  (params (`In Color and Opacity A` :type "Float (single-precision)"))
  (bind (_direction _multiplier) (`Timeline|DamageReticleDisappeardLeft` :!via `PlayFromStart`)
    (:`Update`
      (`Image.SetColorAndOpacity` (`/Game/Blueprints/HUD/BP_HUD.Left_Reticle` (`self.HUDRef`)) (make `LinearColor` 1.0 1.0 1.0 (* _multiplier `In Color and Opacity A`))))))

(event `BottomDamageReticle`
  (params (`In Color and Opacity A` :type "Float (single-precision)"))
  (bind (_direction _multiplier) (`Timeline|DamageReticleDisappearBottom` :!via `PlayFromStart`)
    (:`Update`
      (`Image.SetColorAndOpacity` (`/Game/Blueprints/HUD/BP_HUD.Bottom_Reticle` (`self.HUDRef`)) (make `LinearColor` 1.0 1.0 1.0 (* _multiplier `In Color and Opacity A`))))))

(fn `UserConstructionScript`)