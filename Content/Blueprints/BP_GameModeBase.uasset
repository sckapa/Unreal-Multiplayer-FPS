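; Base game mode that handles player respawning with a killer-tracking death camera.
; RespawnPlayer spawns a DeathCamera at the hit player's transform, possesses it with the player's controller and has it track the killer.
; After a short delay it destroys the camera, then spawns and possesses a new BP_Character at a PlayerStart.
; PlayerStartIndex advances after each spawn and wraps around, cycling spawn points round-robin.
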(event `RespawnPlayer`
  (params (Controller :type "Controller Object Reference") (HitPlayerTransform :type "Transform Structure") (Killer :type "/Game/Blueprints/BP_Character Object Reference"))
  (bind _returnvalue (`|SpawnActorFromClass` "/Game/Blueprints/DeathCamera.DeathCamera_C" HitPlayerTransform "AdjustIfPossibleButAlwaysSpawn" "MultiplyWithRoot" null null))
  (`Controller.Possess` Controller _returnvalue)
  (`/Game/Blueprints/DeathCamera.TrackKiller` _returnvalue Killer)
  (`KismetSystemLibrary.Delay` 3.0)
  (`Controller.UnPossess` Controller)
  (`self.K2_DestroyActor` _returnvalue)
  (bind _outactors (`GameplayStatics.GetAllActorsOfClass` "/Script/Engine.PlayerStart"))
  (bind _returnvalue_2 (`KismetArrayLibrary.Array_Length` _outactors))
  (if (> _returnvalue_2 0)
    (bind _returnvalue_3 (`|SpawnActorFromClass` "/Game/Blueprints/BP_Character.BP_Character_C" (`self.GetTransform` (`|GetArrayItem` _outactors (`self.PlayerStartIndex`))) "AdjustIfPossibleButAlwaysSpawn" "MultiplyWithRoot" null null))
    (`Controller.Possess` Controller _returnvalue_3)
    (bind _result (`/Engine/EditorBlueprintResources/StandardMacros.IncrementInt` (`self.PlayerStartIndex`))
      (:`  `
        (if (>= _result _returnvalue_2)
          (set `self.PlayerStartIndex` 0))))))

(fn `UserConstructionScript`)