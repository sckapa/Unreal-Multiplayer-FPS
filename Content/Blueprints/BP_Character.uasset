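; Player character for a multiplayer shooter, handling movement, look, automatic hitscan fire and timed auto-reload.
; A looping timer fires camera line traces, with damage set by hit component name (head, body, leg) and distance falloff.
; Victims get four-way damage reticle weights from dot products toward the shooter, while OnRep Health updates health text.
; At zero health, the authority destroys the victim after a brief replication delay and requests a GameMode respawn.
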(event `EnhancedInput|/Game/Blueprints/Inputs/IA_MouseY`
  (params (ActionValue :type "Float (double-precision)") (ElapsedSeconds :type "Float (double-precision)") (TriggeredSeconds :type "Float (double-precision)") (InputAction :type "InputAction Object Reference" :default "/Game/Blueprints/Inputs/IA_MouseY.IA_MouseY"))
  ;[1 1 1] Mouse Left & Right
  (:`Triggered`
    (`self.AddControllerYawInput` ActionValue)))

(event `EnhancedInput|/Game/Blueprints/Inputs/IA_MouseX`
  (params (ActionValue :type "Float (double-precision)") (ElapsedSeconds :type "Float (double-precision)") (TriggeredSeconds :type "Float (double-precision)") (InputAction :type "InputAction Object Reference" :default "/Game/Blueprints/Inputs/IA_MouseX.IA_MouseX"))
  ;[1 1 1] Mouse Up & Down
  (:`Triggered`
    (`self.AddControllerPitchInput` ActionValue)))

(event `EnhancedInput|/Game/Blueprints/Inputs/IA_MoveFB`
  (params (ActionValue :type "Float (double-precision)") (ElapsedSeconds :type "Float (double-precision)") (TriggeredSeconds :type "Float (double-precision)") (InputAction :type "InputAction Object Reference" :default "/Game/Blueprints/Inputs/IA_MoveFB.IA_MoveFB"))
  ;[1 1 1] Move forward and backward
  (:`Triggered`
    (`self.AddMovementInput` (`self.GetActorForwardVector`) ActionValue)))

(event `EnhancedInput|/Game/Blueprints/Inputs/IA_MoveSideways`
  (params (ActionValue :type "Float (double-precision)") (ElapsedSeconds :type "Float (double-precision)") (TriggeredSeconds :type "Float (double-precision)") (InputAction :type "InputAction Object Reference" :default "/Game/Blueprints/Inputs/IA_MoveSideways.IA_MoveSideways"))
  ;[1 1 1] Move sideways
  (:`Triggered`
    (`self.AddMovementInput` (`self.GetActorRightVector`) ActionValue)))

(event `SetShooterDataForDmgReticle`
  (params (Shooter :type "/Game/Blueprints/BP_Character Object Reference"))
  (bind _returnvalue (`KismetMathLibrary.Normal` (- (`self.K2_GetActorLocation` Shooter) (`self.K2_GetActorLocation`))))
  ;[1 1 1] Damage Reticle Calculation
  (if (!= _returnvalue (0.0 0.0 0.0))
    (`self.DotWithForward` _returnvalue)
    (`self.DotWithRight` _returnvalue)
    (`self.DotWithBackward` _returnvalue)
    (`self.DotWithLeft` _returnvalue)))

(event `self.ReceiveBeginPlay`
  (bind _asbp_player_controller (cast `/Game/Blueprints/BP_PlayerController` (`GameplayStatics.GetPlayerController` 0)))
  (set `self.PlayerController` _asbp_player_controller)
  (bind _returnvalue (pcsubsystem `EnhancedInputLocalPlayerSubsystem` _asbp_player_controller))
  (`/Engine/EditorBlueprintResources/StandardMacros.IsValid` _returnvalue
    (:`Is Valid`
      (`EnhancedInputSubsystemInterface.AddMappingContext` _returnvalue "/Game/Blueprints/Inputs/InputMappingContext.InputMappingContext" 0 (struct)))))

(event `EnhancedInput|/Game/Blueprints/Inputs/IA_LMB`
  (params (ActionValue :type Boolean) (ElapsedSeconds :type "Float (double-precision)") (TriggeredSeconds :type "Float (double-precision)") (InputAction :type "InputAction Object Reference" :default "/Game/Blueprints/Inputs/IA_LMB.IA_LMB"))
  (bind _shoottimer (`self.ShootTimer`))
  (:`Triggered`
    (if ActionValue
      (bind _returnvalue (`KismetSystemLibrary.K2_SetTimer` null "Shoot" 0.1 true))
      (set `self.ShootTimer` _returnvalue)
      (elif (`KismetSystemLibrary.K2_IsValidTimerHandle` _shoottimer)
        (`KismetSystemLibrary.K2_PauseTimerHandle` _shoottimer)))))

(event `DotWithForward`
  (params (Direction :type "Vector Structure"))
  ;[1 1 1] Damage Reticle Calculation
  (`/Game/Blueprints/BP_PlayerController.TopDamageReticle` (`self.PlayerController`) (`KismetMathLibrary.FClamp` (`KismetMathLibrary.Dot_VectorVector` Direction (`self.GetActorForwardVector`)))))

(event `DotWithBackward`
  (params (Direction :type "Vector Structure"))
  ;[1 1 1] Damage Reticle Calculation
  (`/Game/Blueprints/BP_PlayerController.BottomDamageReticle` (`self.PlayerController`) (`KismetMathLibrary.FClamp` (`KismetMathLibrary.Dot_VectorVector` Direction (`KismetMathLibrary.NegateVector` (`self.GetActorForwardVector`))))))

(event `DotWithRight`
  (params (Direction :type "Vector Structure"))
  ;[1 1 1] Damage Reticle Calculation
  (`/Game/Blueprints/BP_PlayerController.RightDamageReticle` (`self.PlayerController`) (`KismetMathLibrary.FClamp` (`KismetMathLibrary.Dot_VectorVector` Direction (`self.GetActorRightVector`)))))

(event `DotWithLeft`
  (params (Direction :type "Vector Structure"))
  ;[1 1 1] Damage Reticle Calculation
  (`/Game/Blueprints/BP_PlayerController.LeftDamageReticle` (`self.PlayerController`) (`KismetMathLibrary.FClamp` (`KismetMathLibrary.Dot_VectorVector` Direction (`KismetMathLibrary.NegateVector` (`self.GetActorRightVector`))))))

(event `Shoot`
  (if (> (`self.Bullets`) 0)
    (bind _outhit (`self.LineTrace`))
    (`self.BulletCount`)
    (bind (_bblockinghit _binitialoverlap _time _distance _location _impactpoint _normal _impactnormal _physmat _hitactor _hitcomponent) (`GameplayStatics.BreakHitResult` _outhit))
    (bind _asbp_character (cast `/Game/Blueprints/BP_Character` _hitactor))
    (`self.DmgCalculator` _hitcomponent _distance)
    (`self.UpdateHealth` (- (`/Game/Blueprints/BP_Character.Health` _asbp_character) (`self.DeductHealth`)) _asbp_character self)))

(event `Reload`
  (bind _output_get (set `self.Bullets` 30))
  (`/Game/Blueprints/BP_PlayerController.UpdateBullets` (`self.PlayerController`) _output_get))

(event `UpdateHealth`
  (params (NewHealth :type Integer) (ObjRef :type "/Game/Blueprints/BP_Character Object Reference") (Killer :type "/Game/Blueprints/BP_Character Object Reference"))
  (`self.SetShooterDataForDmgReticle` ObjRef Killer)
  (bind _output_get (set `/Game/Blueprints/BP_Character.Health` NewHealth ObjRef))
  (if (<= _output_get 0)
    (`self.CallRespawnInGameMode` (`self.GetController` ObjRef) ObjRef Killer)))

(event `CallRespawnInGameMode`
  (params (Controller :type "Controller Object Reference") (HitObj :type "/Game/Blueprints/BP_Character Object Reference") (Killer :type "/Game/Blueprints/BP_Character Object Reference"))
  (`KismetSystemLibrary.Delay` 0.03) ; Added to make sure health value is replicated before destroying the character
  (`/Engine/EditorBlueprintResources/ActorMacros.Switch Has Authority`
    (:`Authority`
      (`Controller.UnPossess` Controller)
      (set `self.DeadPlayerTransform` (`self.GetTransform` HitObj))
      (`self.K2_DestroyActor` HitObj)
      (`/Game/Blueprints/BP_GameModeBase.RespawnPlayer` (cast `/Game/Blueprints/BP_GameModeBase` (`GameplayStatics.GetGameMode`) :!pure true) Controller (`self.DeadPlayerTransform`) Killer))))

(fn `BulletCount`
  (bind _result (`/Engine/EditorBlueprintResources/StandardMacros.DecrementInt` (`self.Bullets`))
    (:`  `
      (bind _output_get (set `self.Bullets` _result))
      (`/Game/Blueprints/BP_PlayerController.UpdateBullets` (`self.PlayerController`) _output_get)
      (if (<= _output_get 0)
        (`KismetSystemLibrary.K2_SetTimer` null "Reload" 2.5)))))

(fn `DmgCalculator`
  (params (Object :type "Object Object Reference") (Distance :type "Float (double-precision)"))
  (locals (MaxDamage :type "Float (double-precision)") (MaxDistance :type "Float (double-precision)" :default 5000.0) (MinDamage :type "Float (double-precision)" :default 10.0))
  (bind _mindamage (`local.MinDamage`))
  (if (!= (`KismetStringLibrary.FindSubstring` (`KismetSystemLibrary.GetDisplayName` Object) "body") -1)
    (set `local.MaxDamage` 27.0)
    (set `self.DeductHealth` (`KismetMathLibrary.FTrunc` (+ _mindamage (* (- (`local.MaxDamage`) _mindamage) (- 1.0 (`KismetMathLibrary.MultiplyMultiply_FloatFloat` (/ Distance (`local.MaxDistance`)) (`KismetMathLibrary.Conv_IntToDouble` (`self.DamageDropOffFactor`))))))) :!label _label)
    (return)
    (elif (!= (`KismetStringLibrary.FindSubstring` (`KismetSystemLibrary.GetDisplayName` Object) "head") -1)
      (set `local.MaxDamage` 90.0)
      (goto _label)
      (elif (!= (`KismetStringLibrary.FindSubstring` (`KismetSystemLibrary.GetDisplayName` Object) "leg") -1)
        (set `local.MaxDamage` 10.0)
        (goto _label)))))

(fn `LineTrace`
  (returns (OutHit :type "HitResult Structure"))
  (bind _camera (`self.Camera`))
  (bind _returnvalue (`SceneComponent.K2_GetComponentLocation` _camera))
  (bind _outhit (`KismetSystemLibrary.LineTraceSingle` :`Start` _returnvalue :`End` (+ _returnvalue (* (`SceneComponent.GetForwardVector` _camera) 10000.0)) :`TraceChannel` "TraceTypeQuery1" :`DrawDebugType` "ForOneFrame"))
  (return _outhit))

(fn `OnRep_Health`
  (bind _playercontroller (`self.PlayerController`))
  (if (`self.IsLocallyControlled`)
    (if (> (`self.Health`) 0)
      (`/Game/Blueprints/BP_PlayerController.UpdateHealthText` _playercontroller (`self.Health`))
      (else
        (`/Game/Blueprints/BP_PlayerController.UpdateHealthText` _playercontroller 0)))))

(fn `UserConstructionScript`)