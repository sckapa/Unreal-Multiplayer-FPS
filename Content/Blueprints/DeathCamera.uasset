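; DeathCamera is an actor whose camera turns to face a stored Killer, apparently as a death view.
; TrackKiller stores the Killer, and Tick then points the camera straight at it every frame while it is valid.
; StartTrkin plays a timeline that lerps from the actor's rotation to a look-at on the Killer, setting the same camera rotation that Tick also writes.
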(event `TrackKiller`
  (params (Killer :type "/Game/Blueprints/BP_Character Object Reference"))
  (set `self.Killer` Killer))

(event `self.ReceiveTick`
  (params (DeltaSeconds :type "Float (single-precision)"))
  (bind _killer (`self.Killer`))
  (`/Engine/EditorBlueprintResources/StandardMacros.IsValid` _killer
    (:`Is Valid`
      (`SceneComponent.K2_SetWorldRotation` (`self.Camera`) (`KismetMathLibrary.Conv_VectorToRotator` (- (`self.K2_GetActorLocation` _killer) (`self.K2_GetActorLocation`))) false false))))

(event `StartTrkin`
  (`/Engine/EditorBlueprintResources/StandardMacros.IsValid` (`self.Killer`)
    (:`Is Valid`
      (bind (_direction _newtrack_0) (`Timeline|Timeline`)
        (:`Update`
          (`SceneComponent.K2_SetWorldRotation` (`self.Camera`) (`KismetMathLibrary.RLerp` (`self.K2_GetActorRotation`) (`KismetMathLibrary.FindLookAtRotation` (`self.K2_GetActorLocation`) (`self.K2_GetActorLocation` (`self.Killer`))) _newtrack_0) false false))))))

(fn `UserConstructionScript`)